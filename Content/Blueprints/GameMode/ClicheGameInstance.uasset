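; Game instance that keeps player inventory, completed dungeons and first-play/saved-game flags, persisted in one BP_SaveGame slot.
; On Init it loads the slot into its variables, or creates and saves a default object without copying those defaults back.
; SaveGame writes the variables to disk but rebuilds the Keys map with default values instead of copying the player's.
; LoadGame restores from the cached save object without rereading disk.
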(event `self.ReceiveInit`
  ;[1 0 0.5391] Put logic to load saved game
  (`self.InitializeGame`))

(fn `InitializeGame`
  (bind _returnvalue (`GameplayStatics.DoesSaveGameExist` "SaveSlot1"))
  (if _returnvalue
    (bind _returnvalue_2 (`GameplayStatics.LoadGameFromSlot` "SaveSlot1"))
    (bind _asbp_save_game (cast `/Game/Blueprints/SaveGame/BP_SaveGame` _returnvalue_2))
    (set `self.SaveGameSlot` _asbp_save_game)
    (set `self.PlayerItems` (`/Game/Blueprints/SaveGame/BP_SaveGame.PlayerInventory` _asbp_save_game))
    (set `self.DungeonsCompleted` (`/Game/Blueprints/SaveGame/BP_SaveGame.DungeonsCompleted` _asbp_save_game))
    (set `self.isFirstTimePlaying` (`/Game/Blueprints/SaveGame/BP_SaveGame.isFirstTimePlaying` _asbp_save_game))
    (set `self.savedGameLoaded` (`/Game/Blueprints/SaveGame/BP_SaveGame.SavedGame` _asbp_save_game))
    (else
      (bind _returnvalue_3 (`GameplayStatics.CreateSaveGameObject` "/Game/Blueprints/SaveGame/BP_SaveGame.BP_SaveGame_C"))
      (set `/Game/Blueprints/SaveGame/BP_SaveGame.PlayerInventory` (make `/Game/Blueprints/Characters/MainHeroe/Structs/Inventory_Struct` (`|MakeMap` "NewEnumerator0" false "NewEnumerator1" :!type "/Game/Blueprints/Characters/MainHeroe/Enums/KeysEnum Enum") (`|MakeMap` "NewEnumerator0" false "NewEnumerator1" false "NewEnumerator2" false "NewEnumerator3" false "NewEnumerator4" false "NewEnumerator5" false "NewEnumerator6" :!type "/Game/Blueprints/Characters/MainHeroe/Enums/HeroeEquipEnum Enum") 0 200 200) _returnvalue_3)
      (set `/Game/Blueprints/SaveGame/BP_SaveGame.DungeonsCompleted` (`|MakeMap` "NewEnumerator0" false "NewEnumerator1" false "NewEnumerator2" false "NewEnumerator3" false "NewEnumerator4" :!type "/Game/Blueprints/Enums/DungeonsEnum Enum") _returnvalue_3)
      (set `/Game/Blueprints/SaveGame/BP_SaveGame.isFirstTimePlaying` true _returnvalue_3)
      (set `/Game/Blueprints/SaveGame/BP_SaveGame.SavedGame` false _returnvalue_3)
      (`GameplayStatics.SaveGameToSlot` _returnvalue_3 "SaveSlot1")
      (set `self.SaveGameSlot` _returnvalue_3))))

(fn `LoadGame`
  (bind _savegameslot (`self.SaveGameSlot`))
  (bind _returnvalue (`GameplayStatics.DoesSaveGameExist` "SaveSlot1"))
  (if _returnvalue
    (set `self.PlayerItems` (`/Game/Blueprints/SaveGame/BP_SaveGame.PlayerInventory` _savegameslot))
    (set `self.DungeonsCompleted` (`/Game/Blueprints/SaveGame/BP_SaveGame.DungeonsCompleted` _savegameslot))
    (set `self.isFirstTimePlaying` (`/Game/Blueprints/SaveGame/BP_SaveGame.isFirstTimePlaying` _savegameslot))
    (set `self.savedGameLoaded` (`/Game/Blueprints/SaveGame/BP_SaveGame.SavedGame` _savegameslot))))

(fn `SaveGame`
  (bind _savegameslot (`self.SaveGameSlot`))
  (bind (_keys _equipment _coins _bluebulletsammo _redbulletsammo) (break `/Game/Blueprints/Characters/MainHeroe/Structs/Inventory_Struct` (`self.PlayerItems`)))
  (bind _returnvalue (`GameplayStatics.DoesSaveGameExist` "SaveSlot1"))
  (if _returnvalue
    (set `/Game/Blueprints/SaveGame/BP_SaveGame.PlayerInventory` (make `/Game/Blueprints/Characters/MainHeroe/Structs/Inventory_Struct` (`|MakeMap` "NewEnumerator0" false "NewEnumerator1" :!type "/Game/Blueprints/Characters/MainHeroe/Enums/KeysEnum Enum") _equipment _coins _bluebulletsammo _redbulletsammo) _savegameslot)
    (set `/Game/Blueprints/SaveGame/BP_SaveGame.DungeonsCompleted` (`self.DungeonsCompleted`) _savegameslot)
    (set `/Game/Blueprints/SaveGame/BP_SaveGame.isFirstTimePlaying` (`self.isFirstTimePlaying`) _savegameslot)
    (set `/Game/Blueprints/SaveGame/BP_SaveGame.SavedGame` (`self.savedGameLoaded`) _savegameslot)
    (`GameplayStatics.SaveGameToSlot` _savegameslot "SaveSlot1")))