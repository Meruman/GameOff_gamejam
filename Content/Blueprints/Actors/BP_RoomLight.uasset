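; BP_RoomLight is a placeable room light that turns on only while the player is inside its trigger volume.
; Box overlap begin and end events show or hide the PointLight for actors tagged HeroPlayer.
; The construction script applies the box extent and the light's attenuation radius, source radius and intensity from variables, so each instance can be sized and tuned.
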(event `self.Box.OnComponentBeginOverlap`
  (params (OverlappedComponent :type "PrimitiveComponent Object Reference") (OtherActor :type "Actor Object Reference") (OtherComp :type "PrimitiveComponent Object Reference") (OtherBodyIndex :type Integer) (bFromSweep :type Boolean) (SweepResult :type "HitResult Structure (by ref)"))
  (if (`self.ActorHasTag` OtherActor "HeroPlayer")
    (`SceneComponent.SetVisibility` (`self.PointLight`) true false)))

(event `self.Box.OnComponentEndOverlap`
  (params (OverlappedComponent :type "PrimitiveComponent Object Reference") (OtherActor :type "Actor Object Reference") (OtherComp :type "PrimitiveComponent Object Reference") (OtherBodyIndex :type Integer))
  (if (`self.ActorHasTag` OtherActor "HeroPlayer")
    (`SceneComponent.SetVisibility` (`self.PointLight`) false false)))

(fn `UserConstructionScript`
  (bind _pointlight (`self.PointLight`))
  (`BoxComponent.SetBoxExtent` (`self.Box`) (`self.boxSize`) true)
  (`LocalLightComponent.SetAttenuationRadius` _pointlight (`self.AttenuationRadio`))
  (`PointLightComponent.SetSourceRadius` _pointlight (`self.SourceRadio`))
  (`LightComponent.SetIntensity` (`self.PointLight`) (`self.Intensity`)))