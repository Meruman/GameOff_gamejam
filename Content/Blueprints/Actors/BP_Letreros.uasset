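; BP_Letreros is a sign actor that reveals paper and poster props as dungeons are completed.
; Shortly after BeginPlay, it reads the DungeonsCompleted map from ClicheGameInstance and unhides a separate pair of props for each of four completed dungeons.
; The ForceDisplay flag skips these checks and shows every prop.
; Visibility is evaluated only once, and the script never re-hides props.
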(event `self.ReceiveBeginPlay`
  (bind _dungeonscompleted (`/Game/Blueprints/GameMode/ClicheGameInstance.DungeonsCompleted` (cast `/Game/Blueprints/GameMode/ClicheGameInstance` (`GameplayStatics.GetGameInstance`) :!pure true)))
  (`KismetSystemLibrary.Delay` 0.2)
  (if (`self.ForceDisplay`)
    (`SceneComponent.SetHiddenInGame` (`self.SM_PROP_paper_01`) false false)
    (`SceneComponent.SetHiddenInGame` (`self.SM_PROP_paper_05`) false false)
    (`SceneComponent.SetHiddenInGame` (`self.SM_PROP_poster_02`) false false)
    (`SceneComponent.SetHiddenInGame` (`self.SM_PROP_paper_03`) false false)
    (`SceneComponent.SetHiddenInGame` (`self.SM_PROP_paper_06`) false false)
    (`SceneComponent.SetHiddenInGame` (`self.SM_PROP_poster_01`) false false)
    (`SceneComponent.SetHiddenInGame` (`self.SM_PROP_paper_04`) false false)
    (`SceneComponent.SetHiddenInGame` (`self.SM_PROP_paper_02`) false false)
    (else
      (`|ExecutionSequence`
        (:`then_0`
          (if (`BlueprintMapLibrary.Map_Find` _dungeonscompleted "NewEnumerator0")
            (`SceneComponent.SetHiddenInGame` (`self.SM_PROP_paper_01`) false false)
            (`SceneComponent.SetHiddenInGame` (`self.SM_PROP_paper_05`) false false)))
        (:`then_1`
          (if (`BlueprintMapLibrary.Map_Find` _dungeonscompleted "NewEnumerator1")
            (`SceneComponent.SetHiddenInGame` (`self.SM_PROP_poster_02`) false false)
            (`SceneComponent.SetHiddenInGame` (`self.SM_PROP_paper_03`) false false)))
        (:`then_2`
          (if (`BlueprintMapLibrary.Map_Find` _dungeonscompleted "NewEnumerator2")
            (`SceneComponent.SetHiddenInGame` (`self.SM_PROP_paper_06`) false false)
            (`SceneComponent.SetHiddenInGame` (`self.SM_PROP_poster_01`) false false)))
        (:`then_3`
          (if (`BlueprintMapLibrary.Map_Find` _dungeonscompleted "NewEnumerator3")
            (`SceneComponent.SetHiddenInGame` (`self.SM_PROP_paper_04`) false false)
            (`SceneComponent.SetHiddenInGame` (`self.SM_PROP_paper_02`) false false)))))))

(fn `UserConstructionScript`)