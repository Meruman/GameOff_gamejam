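; BP_MoonLockedDoor is a double door that opens for the hero only when their inventory holds the required key.
; Entering DoorTrigger checks the key, then plays the DoorSlide timeline, swinging both leaves in opposite yaw with a sound.
; The first successful use also destroys the ChildActor component.
; Leaving the trigger reverses the timeline and plays the close sound without checking the key; CheckOpenDoor is an empty stub.
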(event `self.ReceiveBeginPlay`
  (bind _doorright (`self.DoorRight`))
  (bind _doorleft (`self.DoorLeft`))
  (set `self.DoorLeftInitialRotation` (`SceneComponent.RelativeRotation` _doorleft))
  (set `self.DoorRightInitialRotation` (`SceneComponent.RelativeRotation` _doorright))
  (set `self.Door1Offset` (`SceneComponent.RelativeLocation` _doorright))
  (set `self.Door2Offset` (`SceneComponent.RelativeLocation` _doorleft))
  (bind (_direction _openratio) (`Timeline|DoorSlide` :!via `Stop` :!label _label)
    (:`Update`
      (bind _returnvalue (* _openratio 110.0))
      (`SceneComponent.K2_SetRelativeRotation` (`self.DoorRight`) (`KismetMathLibrary.MakeRotator` 0.0 0.0 _returnvalue) false false)
      (`SceneComponent.K2_SetRelativeRotation` (`self.DoorLeft`) (`KismetMathLibrary.MakeRotator` 0.0 0.0 (* _returnvalue -1.0)) false false))))

(event `PlayFromStart`
  (goto _label))

(event `ReverseFromEnd`
  (goto _label :!via `Reverse`))

(event `OpenDoor`
  (`self.PlayFromStart`)
  (`GameplayStatics.PlaySoundAtLocation` "/Game/Everything_Bundle/Ultimate_SFX/Survival_Sound_Kit_HD_Remake/Wavs/Door_Open_2.Door_Open_2" (`self.K2_GetActorLocation`) (struct) 1.0 1.0 0.0 null null null null))

(event `CloseDoor`
  (`self.ReverseFromEnd`)
  (`GameplayStatics.PlaySoundAtLocation` "/Game/Everything_Bundle/Ultimate_SFX/Survival_Sound_Kit_HD_Remake/Wavs/Door_Close_3.Door_Close_3" (`self.K2_GetActorLocation`) (struct) 1.0 1.0 0.0 null null null null))

(event `self.DoorTrigger.OnComponentBeginOverlap`
  (params (OverlappedComponent :type "PrimitiveComponent Object Reference") (OtherActor :type "Actor Object Reference") (OtherComp :type "PrimitiveComponent Object Reference") (OtherBodyIndex :type Integer) (bFromSweep :type Boolean) (SweepResult :type "HitResult Structure (by ref)"))
  (if (`self.ActorHasTag` OtherActor "HeroPlayer")
    (bind _ashero_character (cast `/Game/Blueprints/Characters/BaseClasses/HeroCharacter` OtherActor))
    (if (`BlueprintMapLibrary.Map_Find` (`.Keys_4_3AD3410D406BE811A81684A246E373C3` (break `/Game/Blueprints/Characters/MainHeroe/Structs/Inventory_Struct` (`/Game/Blueprints/Characters/BaseClasses/HeroCharacter.Inventory` _ashero_character))) (`self.RequiredKey`))
      (`self.OpenDoor`)
      (`/Engine/EditorBlueprintResources/StandardMacros.DoOnce` false
        (:`Completed`
          (`KismetSystemLibrary.PrintString` "Key used")
          (`ActorComponent.K2_DestroyComponent` (`self.ChildActor`))))
      (else
        (`KismetSystemLibrary.PrintString` "No key for this door")))))

(event `self.DoorTrigger.OnComponentEndOverlap`
  (params (OverlappedComponent :type "PrimitiveComponent Object Reference") (OtherActor :type "Actor Object Reference") (OtherComp :type "PrimitiveComponent Object Reference") (OtherBodyIndex :type Integer))
  (if (`self.ActorHasTag` OtherActor "HeroPlayer")
    (`self.CloseDoor`)))

(fn `CheckOpenDoor`)

(fn `UserConstructionScript`)