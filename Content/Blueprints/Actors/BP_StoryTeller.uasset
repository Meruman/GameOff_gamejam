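; BP_StoryTeller plays a scripted dialogue sequence from the TextDialog data table in a StoryTellerWidget, showing the princess, fairy or enemy portrait for each line.
; RunStoryTeller advances through rows after a delay and calls AllTextDone when finished.
; DisplayText types letters using a self-restarting timer, and a debounced Q press completes the current line.
; The sixth line is hard-coded to swap Fairy1 for Fairy2 and a Cage.
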(event `SetupStoryTeller`
  (`KismetSystemLibrary.Delay` 0.5)
  (bind _returnvalue (`|CreateWidget` "/Game/Blueprints/MainMenu/StoryTellerWidget.StoryTellerWidget_C" (`GameplayStatics.GetPlayerController` 0) :!label _label))
  (`UserWidget.AddToViewport` _returnvalue -1)
  (set `self.Border Conversation` (`/Game/Blueprints/MainMenu/StoryTellerWidget.BorderConversation` _returnvalue))
  (set `self.Conversation Display Text` (`/Game/Blueprints/MainMenu/StoryTellerWidget.ConversationDisplayText` _returnvalue))
  (set `self.Enemy Image` (`/Game/Blueprints/MainMenu/StoryTellerWidget.Enemy_Image` _returnvalue))
  (set `self.Fairy Image` (`/Game/Blueprints/MainMenu/StoryTellerWidget.Fairy_Image` _returnvalue))
  (set `self.Princess Image` (`/Game/Blueprints/MainMenu/StoryTellerWidget.Princess_Image` _returnvalue))
  (`self.EnableInput` (`GameplayStatics.GetPlayerController` 0) null)
  (set `self.DialogWidget` _returnvalue))

(event `self.ReceiveBeginPlay`
  (`KismetSystemLibrary.Delay` 0.5)
  (goto _label))

(event `StartStoryTeller`
  (`self.RunStoryTeller`))

(event `RunStoryTeller`
  (bind _textdialog (`self.TextDialog`))
  (bind _result (`/Engine/EditorBlueprintResources/StandardMacros.IncrementInt` (`self.IndexIterator`))
    (:`  `
      (set `self.IndexIterator` _result)
      (bind _outrownames (`DataTableFunctionLibrary.GetDataTableRowNames` _textdialog))
      (set `self.DialogRowNames` _outrownames)
      (if (>= (`self.IndexIterator`) (`DataTableFL.GetDataTableSize` _textdialog))
        (`KismetSystemLibrary.Delay` (`self.DelayBetweenLines`))
        (`TextBlock.SetText` (`self.Conversation Display Text`) "")
        (`Widget.SetVisibility` (`self.Princess Image`) "Collapsed")
        (`Widget.SetVisibility` (`self.Fairy Image`) "Collapsed")
        (`Widget.SetVisibility` (`self.Enemy Image`) "Collapsed")
        (set `self.IndexIterator` -1)
        (`Widget.RemoveFromParent` (`self.DialogWidget`))
        (`self.AllTextDone`)
        (else
          (if (> (`self.IndexIterator`) 0)
            (`KismetSystemLibrary.Delay` (`self.DelayBetweenLines`))
            (`Widget.SetVisibility` (`self.Princess Image`) "Hidden")
            (`Widget.SetVisibility` (`self.Fairy Image`) "Hidden")
            (`Widget.SetVisibility` (`self.Enemy Image`) "Hidden")
            (else
              (`Widget.SetVisibility` (`self.Border Conversation`) "Visible")))
          (`TextBlock.SetText` (`self.Conversation Display Text`) "")
          (if (== (`self.IndexIterator`) 5)
            (`/Engine/EditorBlueprintResources/StandardMacros.IsValid` (`self.Fairy1`)
              (:`Is Valid`
                (`self.SetActorHiddenInGame` (`self.Fairy2`) false)
                (`self.SetActorHiddenInGame` (`self.Cage`) false)
                (`self.SetActorHiddenInGame` (`self.Fairy1`) true))))
          (set `self.FinishTextNow` false)
          (bind _returnvalue (`|GetDataTableRow` (`self.TextDialog`) (`|GetArrayItem` (`self.DialogRowNames`) (`self.IndexIterator`)))
            (:`then`
              (bind (_charactername _dialog) (break `/Game/Blueprints/Struct/Characters_Story` _returnvalue))
              (set `self.CurrentStringToDisplay` (`KismetTextLibrary.Conv_TextToString` _dialog))
              (switch `/Game/Blueprints/Enums/CharactersEnum` _charactername
                (:`NewEnumerator0`
                  (`Widget.SetVisibility` (`self.Princess Image`) "Visible"))
                (:`NewEnumerator1`
                  (`Widget.SetVisibility` (`self.Enemy Image`) "Visible"))
                (:`NewEnumerator2`
                  (`Widget.SetVisibility` (`self.Fairy Image`) "Visible")))
              (`self.DisplayText`))))))))

(event `FinishCurrentLineNow`
  (set `self.FinishTextNow` true))

(event `Key|Q`
  (params (Key :type "Key Structure"))
  (:`Pressed`
    (`/Engine/EditorBlueprintResources/StandardMacros.DoOnce` false :!label _label_2
      (:`Completed`
        (`self.FinishCurrentLineNow`)
        (`KismetSystemLibrary.Delay` 0.3)
        (goto _label_2 :!via `Reset`)))))

(fn `DisplayText`
  (bind _returnvalue (`KismetTextLibrary.Conv_TextToString` (`TextBlock.GetText` (`self.Conversation Display Text`))))
  (`TextBlock.SetText` (`self.Conversation Display Text`) (`KismetTextLibrary.Conv_StringToText` (`KismetStringLibrary.Concat_StrStr` _returnvalue (`KismetStringLibrary.GetSubstring` (`self.CurrentStringToDisplay`) (`KismetStringLibrary.Len` _returnvalue)))))
  (if (`self.FinishTextNow`)
    (`TextBlock.SetText` (`self.Conversation Display Text`) (`KismetTextLibrary.Conv_StringToText` (`self.CurrentStringToDisplay`)))
    (`self.RunStoryTeller`)
    (elif (`KismetTextLibrary.EqualEqual_TextText` (`TextBlock.GetText` (`self.Conversation Display Text`)) (`KismetTextLibrary.Conv_StringToText` (`self.CurrentStringToDisplay`)))
      (`self.RunStoryTeller`)
      (else
        (`KismetSystemLibrary.K2_SetTimer` null "DisplayText" (`self.DelayBetweenLetters`))))))

(fn `UserConstructionScript`)