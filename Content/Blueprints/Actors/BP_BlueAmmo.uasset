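; BP_BlueAmmo is a pickup actor that gives blue bullets to the hero player.
; When its Sphere overlaps an actor tagged HeroPlayer, it casts to HeroCharacter_Main and calls AddAmmo with the configured amount.
; It then spawns an energy particle system at its location and destroys itself.
; The construction script sizes the trigger sphere from the CollisionRadius variable.
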(event `self.Sphere.OnComponentBeginOverlap`
  (params (OverlappedComponent :type "PrimitiveComponent Object Reference") (OtherActor :type "Actor Object Reference") (OtherComp :type "PrimitiveComponent Object Reference") (OtherBodyIndex :type Integer) (bFromSweep :type Boolean) (SweepResult :type "HitResult Structure (by ref)"))
  (bind (_returnvalue_location _returnvalue_rotation) (`KismetMathLibrary.BreakTransform` (`self.GetTransform`)))
  (if (`self.ActorHasTag` OtherActor "HeroPlayer")
    (bind _ashero_character_main (cast `/Game/Blueprints/Characters/MainHeroe/HeroCharacter_Main` OtherActor))
    (`/Game/Blueprints/Characters/MainHeroe/HeroCharacter_Main.AddAmmo` _ashero_character_main true (`self.Ammo Amount`))
    (`NiagaraFunctionLibrary.SpawnSystemAtLocation` "/Game/sA_PickupSet_1/Fx/NiagaraSystems/NS_Energy_2.NS_Energy_2" _returnvalue_location _returnvalue_rotation (2.0 2.0 2.0))
    (`self.K2_DestroyActor`)))

(fn `UserConstructionScript`
  (`parent.UserConstructionScript`)
  (`SphereComponent.SetSphereRadius` (`self.Sphere`) (`self.CollisionRadius`) true))