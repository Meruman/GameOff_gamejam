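; Large double dungeon door that swings open when an actor tagged HeroPlayer enters its trigger and closes when that actor leaves.
; The DoorSlide timeline yaws the two leaves in opposite directions, setting absolute relative rotations rather than offsets from the starting pose.
; Opening plays from the start and closing reverses from the end, so an interrupted swing snaps to an endpoint.
; Initial rotations and offsets are cached on BeginPlay but never read.
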(event `self.ReceiveBeginPlay`
  (bind _doorright (`self.DoorRight`))
  (bind _doorleft (`self.DoorLeft`))
  (set `self.DoorLeftInitialRotation` (`SceneComponent.RelativeRotation` _doorleft))
  (set `self.DoorRightInitialRotation` (`SceneComponent.RelativeRotation` _doorright))
  (set `self.Door1Offset` (`SceneComponent.RelativeLocation` _doorright))
  (set `self.Door2Offset` (`SceneComponent.RelativeLocation` _doorleft))
  (bind (_direction _openratio) (`Timeline|DoorSlide` :`NewTime` 0.0 :!via `Stop` :!label _label)
    (:`Update`
      (bind _returnvalue (* _openratio 110.0))
      (`SceneComponent.K2_SetRelativeRotation` (`self.DoorRight`) (`KismetMathLibrary.MakeRotator` 0.0 0.0 _returnvalue) false false)
      (`SceneComponent.K2_SetRelativeRotation` (`self.DoorLeft`) (`KismetMathLibrary.MakeRotator` 0.0 0.0 (* _returnvalue -1.0)) false false))))

(event `PlayFromStart`
  (goto _label :!via `PlayFromStart`))

(event `ReverseFromEnd`
  (goto _label :!via `ReverseFromEnd`))

(event `OpenDoor`
  (`self.PlayFromStart`))

(event `CloseDoor`
  (`self.ReverseFromEnd`))

(event `self.DoorTrigger.OnComponentBeginOverlap`
  (params (OverlappedComponent :type "PrimitiveComponent Object Reference") (OtherActor :type "Actor Object Reference") (OtherComp :type "PrimitiveComponent Object Reference") (OtherBodyIndex :type Integer) (bFromSweep :type Boolean) (SweepResult :type "HitResult Structure (by ref)"))
  (if (`self.ActorHasTag` OtherActor "HeroPlayer")
    (`self.OpenDoor`)))

(event `self.DoorTrigger.OnComponentEndOverlap`
  (params (OverlappedComponent :type "PrimitiveComponent Object Reference") (OtherActor :type "Actor Object Reference") (OtherComp :type "PrimitiveComponent Object Reference") (OtherBodyIndex :type Integer))
  (if (`self.ActorHasTag` OtherActor "HeroPlayer")
    (`self.CloseDoor`)))

(fn `UserConstructionScript`)