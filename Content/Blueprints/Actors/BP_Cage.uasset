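; BP_Cage is a dungeon cage actor that opens when its linked boss dies and ends the dungeon when the hero enters it.
; On BeginPlay it binds to the boss death event, which destroys the lock component and plays a timeline that swings the door open while enabling the trigger box collision.
; A HeroPlayer-tagged actor overlapping the box calls DungeonCompleted on the hero character, passing the Winning_Level name.
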(event `self.ReceiveBeginPlay`
  (add `/Game/Blueprints/Characters/BaseClasses/EnemyCharacter.Boss_Dead` (`self.Boss`) (delegate `BossDead`)))

(event `BossDead`
  (`ActorComponent.K2_DestroyComponent` (`self.BP_PROP_lock_dungeon`))
  (bind (_direction _newtrack_0) (`Timeline|OpenDoor`)
    (:`Update`
      (`SceneComponent.K2_SetRelativeRotation` (`self.SM_PROP_cage_door_01_dungeon`) (`KismetMathLibrary.RLerp` (struct) (struct :`Yaw` -120.0) _newtrack_0) false false)
      (`PrimitiveComponent.SetCollisionEnabled` (`self.Box`) "QueryAndPhysics"))))

(event `self.Box.OnComponentBeginOverlap`
  (params (OverlappedComponent :type "PrimitiveComponent Object Reference") (OtherActor :type "Actor Object Reference") (OtherComp :type "PrimitiveComponent Object Reference") (OtherBodyIndex :type Integer) (bFromSweep :type Boolean) (SweepResult :type "HitResult Structure (by ref)"))
  (if (`self.ActorHasTag` OtherActor "HeroPlayer")
    (`/Game/Blueprints/Characters/MainHeroe/HeroCharacter_Main.DungeonCompleted` (cast `/Game/Blueprints/Characters/MainHeroe/HeroCharacter_Main` OtherActor :!pure true) "NewEnumerator4" "Winning_Level")))

(fn `UserConstructionScript`)