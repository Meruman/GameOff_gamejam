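; BP_DungeonDone_Teleport is the dungeon exit actor that rewards the hero and completes the dungeon.
; An Activate event enables the sphere's collision, unhides the actor and coin, starts its audio and begins rotating movement.
; When an actor tagged HeroPlayer overlaps the sphere, it adds MoneyToAdd to that hero and calls DungeonCompleted with DungeonLevel and the Starter_village level name.
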(event `self.Sphere.OnComponentBeginOverlap`
  (params (OverlappedComponent :type "PrimitiveComponent Object Reference") (OtherActor :type "Actor Object Reference") (OtherComp :type "PrimitiveComponent Object Reference") (OtherBodyIndex :type Integer) (bFromSweep :type Boolean) (SweepResult :type "HitResult Structure (by ref)"))
  (if (`self.ActorHasTag` OtherActor "HeroPlayer")
    (`/Game/Blueprints/Characters/MainHeroe/HeroCharacter_Main.IncreaseMoney` (cast `/Game/Blueprints/Characters/MainHeroe/HeroCharacter_Main` OtherActor :!pure true) (`self.MoneyToAdd`))
    (`/Game/Blueprints/Characters/MainHeroe/HeroCharacter_Main.DungeonCompleted` (cast `/Game/Blueprints/Characters/MainHeroe/HeroCharacter_Main` (`GameplayStatics.GetPlayerCharacter` 0) :!pure true) (`self.DungeonLevel`) "Starter_village")))

(event `Activate`
  (bind _audio (`self.Audio`))
  (`PrimitiveComponent.SetCollisionEnabled` (`self.Sphere`) "QueryAndPhysics")
  (`self.SetActorHiddenInGame` self false)
  (`ActorComponent.Activate` _audio false)
  (`AudioComponent.Play` _audio 0.0)
  (`SceneComponent.SetHiddenInGame` (`self.Coin`) false false)
  (`SceneComponent.SetHiddenInGame` (`self.Scene`) false false)
  (`ActorComponent.Activate` (`self.RotatingMovement`) false))

(fn `UserConstructionScript`
  (`parent.UserConstructionScript`)
  (`AudioComponent.Stop` (`self.Audio`)))