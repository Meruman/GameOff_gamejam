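; BP_HealingItem is a health pickup actor for the hero player.
; When an actor tagged HeroPlayer overlaps its Sphere, it casts to ClicheBaseCharacter, restores a fixed amount of health, spawns the NS_Healing_3 effect at its location and destroys itself.
; The construction script applies the SphereSize variable to the sphere's radius, so the pickup range is adjustable.
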(event `self.Sphere.OnComponentBeginOverlap`
  (params (OverlappedComponent :type "PrimitiveComponent Object Reference") (OtherActor :type "Actor Object Reference") (OtherComp :type "PrimitiveComponent Object Reference") (OtherBodyIndex :type Integer) (bFromSweep :type Boolean) (SweepResult :type "HitResult Structure (by ref)"))
  (bind (_returnvalue_location _returnvalue_rotation) (`KismetMathLibrary.BreakTransform` (`self.GetTransform`)))
  (if (`self.ActorHasTag` OtherActor "HeroPlayer")
    (bind _ascliche_base_character (cast `/Game/Blueprints/Characters/BaseClasses/ClicheBaseCharacter` OtherActor))
    (`/Game/Blueprints/Characters/BaseClasses/ClicheBaseCharacter.RecoverHealth` _ascliche_base_character 10.0)
    (`NiagaraFunctionLibrary.SpawnSystemAtLocation` "/Game/sA_PickupSet_1/Fx/NiagaraSystems/NS_Healing_3.NS_Healing_3" _returnvalue_location _returnvalue_rotation (2.0 2.0 2.0))
    (`self.K2_DestroyActor`)))

(fn `UserConstructionScript`
  (`parent.UserConstructionScript`)
  (`SphereComponent.SetSphereRadius` (`self.Sphere`) (`self.SphereSize`) true))