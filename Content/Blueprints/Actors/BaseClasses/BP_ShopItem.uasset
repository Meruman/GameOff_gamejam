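; Base shop item actor that displays a piece of equipment the hero can buy with coins.
; The construction script sets up its mesh, particle, rotation, spotlight and trigger box from per-instance settings.
; Box overlap registers it as the hero's interact target and toggles the prompt.
; Interacting checks the price, updates inventory, HUD and equipment, then destroys the item; YellowBullets also starts the storyteller, and insufficient coins play an error sound.
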(event `self.ReceiveBeginPlay`)

(event `self.Box.OnComponentBeginOverlap`
  (params (OverlappedComponent :type "PrimitiveComponent Object Reference") (OtherActor :type "Actor Object Reference") (OtherComp :type "PrimitiveComponent Object Reference") (OtherBodyIndex :type Integer) (bFromSweep :type Boolean) (SweepResult :type "HitResult Structure (by ref)"))
  (bind _interacttext (`self.InteractText`))
  (if (`self.ActorHasTag` OtherActor "HeroPlayer")
    (`/Engine/EditorBlueprintResources/StandardMacros.DoOnce` false :!label _label
      (:`Completed`
        (bind _ashero_character_main (cast `/Game/Blueprints/Characters/MainHeroe/HeroCharacter_Main` OtherActor))
        (set `/Game/Blueprints/Characters/MainHeroe/HeroCharacter_Main.ActorToInteract` self _ashero_character_main)
        (set `self.HeroCharacterMain` _ashero_character_main)
        (`self.SetActorHiddenInGame` _interacttext false)
        (goto _label_2 :!via `Reset`)))))

(event `self.Box.OnComponentEndOverlap`
  (params (OverlappedComponent :type "PrimitiveComponent Object Reference") (OtherActor :type "Actor Object Reference") (OtherComp :type "PrimitiveComponent Object Reference") (OtherBodyIndex :type Integer))
  (if (`self.ActorHasTag` OtherActor "HeroPlayer")
    (`/Engine/EditorBlueprintResources/StandardMacros.DoOnce` false :!label _label_2
      (:`Completed`
        (bind _ashero_character_main (cast `/Game/Blueprints/Characters/MainHeroe/HeroCharacter_Main` OtherActor))
        (set `/Game/Blueprints/Characters/MainHeroe/HeroCharacter_Main.ActorToInteract` null _ashero_character_main)
        (`self.SetActorHiddenInGame` (`self.InteractText`) true)
        (goto _label :!via `Reset`)))))

(event `/Game/Blueprints/Actors/Interfaces/PickupInterface.Interact`
  (`self.Purchase`))

(event `/Game/Blueprints/Actors/Interfaces/PickupInterface.Deinteract`)

(fn `Purchase`
  (bind _price (`self.Price`))
  (bind _herocharactermain (`self.HeroCharacterMain`))
  (bind _inventory (`/Game/Blueprints/Characters/BaseClasses/HeroCharacter.Inventory` (`self.HeroCharacterMain`)))
  (bind ((`Coins_12_F7B4B0F44C4F5718964563A5A9D86F15` _coins)) (break `/Game/Blueprints/Characters/MainHeroe/Structs/Inventory_Struct` _inventory))
  (bind ((`Equipment_9_BBF199E7467EC702B9D72F862FA01E39` _equipment)) (break `/Game/Blueprints/Characters/MainHeroe/Structs/Inventory_Struct` _inventory))
  (if (>= _coins _price)
    (`BlueprintMapLibrary.Map_Add` _equipment (`self.EquipmentToShow`) true)
    (`/Game/Blueprints/Characters/MainHeroe/HeroCharacter_Main.ChangeInventory` _herocharactermain true (make `/Game/Blueprints/Characters/MainHeroe/Structs/Inventory_Struct` :`Equipment` _equipment :`Coins` (- _coins _price)))
    (`/Game/Blueprints/HUD/HUD_MainCharacter.ChangeCoins` (cast `/Game/Blueprints/HUD/HUD_MainCharacter` (`/Game/Blueprints/Characters/BaseClasses/HeroCharacter.HealthWidgetReference` _herocharactermain) :!pure true) (`.Coins_12_F7B4B0F44C4F5718964563A5A9D86F15` (break `/Game/Blueprints/Characters/MainHeroe/Structs/Inventory_Struct` (`/Game/Blueprints/Characters/BaseClasses/HeroCharacter.Inventory` _herocharactermain))))
    (`/Game/Blueprints/Characters/MainHeroe/HeroCharacter_Main.UpdateEquipment` _herocharactermain)
    (if (`|EnumEquality` (`self.EquipmentToShow`) "NewEnumerator6")
      (bind _outactors (`GameplayStatics.GetAllActorsOfClass` "/Game/Blueprints/Actors/BP_StoryTeller.BP_StoryTeller_C"))
      (`/Game/Blueprints/Actors/BP_StoryTeller.StartStoryTeller` (`|GetArrayItem` _outactors)))
    (`GameplayStatics.PlaySoundAtLocation` "/Game/Everything_Bundle/Ultimate_SFX/UI_Item_Sounds_HD_Remake/Wavs/Item_purchase_5.Item_purchase_5" (`self.K2_GetActorLocation`) (struct) 1.0 1.0 0.0 null null null null)
    (`self.K2_DestroyActor`)
    (else
      (`GameplayStatics.PlaySoundAtLocation` "/Game/Everything_Bundle/Ultimate_SFX/UI_Item_Sounds_HD_Remake/Wavs/Error_Sound_22.Error_Sound_22" (`self.K2_GetActorLocation`) (struct) 1.0 1.0 0.0 null null null null))))

(fn `UserConstructionScript`
  (bind _spotlight (`self.SpotLight`))
  (bind _skeletalmesh (`self.SkeletalMesh`))
  (set `RotatingMovementComponent.RotationRate` (`self.ItemRotationRate`) (`self.RotatingMovement`))
  (`NiagaraComponent.SetAsset` (`self.BulletParticleEffect`) (`self.BulletParticle`) true)
  (`BoxComponent.SetBoxExtent` (`self.Box`) (`self.BoxExtent`) true)
  (`StaticMeshComponent.SetStaticMesh` (`self.StaticMesh`) (`self.ItemMesh`))
  (`SceneComponent.K2_AddLocalOffset` (`self.SkeletalMesh`) (`self.Location offset`) false false)
  (`SceneComponent.K2_AddLocalRotation` (`self.StaticMesh`) (`self.StaticmeshRotation`) false false)
  (`SceneComponent.K2_AddLocalOffset` (`self.StaticMesh`) (`self.StaticMeshLocationOffset`) false false)
  (`SpotLightComponent.SetInnerConeAngle` _spotlight (`self.SpotlightInnerConeAngle`))
  (`SpotLightComponent.SetOuterConeAngle` _spotlight (`self.SpotlightOuterConeAngle`))
  (`LightComponent.SetLightColor` _spotlight (`self.New Light Color`) true)
  (`LocalLightComponent.SetAttenuationRadius` _spotlight (`self.LightAttenuationRadius`))
  (`LightComponent.SetIntensity` _spotlight (`self.LightIntensity`))
  (`SceneComponent.SetRelativeScale3D` (`self.SkeletalMesh`) (`self.MeshScale`))
  (if (not (`SkeletalMeshComponent.HasValidAnimationInstance` (`self.SkeletalMesh`)))
    (switch `/Game/Blueprints/Characters/MainHeroe/Enums/HeroeEquipEnum` (`self.EquipmentToShow`)
      (:`NewEnumerator0`
        (`SkinnedMeshComponent.SetSkinnedAssetAndUpdate` _skeletalmesh "/Game/Cyberman/Mesh/SK_Scapular.SK_Scapular" true))
      (:`NewEnumerator1`
        (`SkinnedMeshComponent.SetSkinnedAssetAndUpdate` _skeletalmesh "/Game/Cyberman/Mesh/SK_Mask.SK_Mask" true))
      (:`NewEnumerator3`
        (`SkinnedMeshComponent.SetSkinnedAssetAndUpdate` _skeletalmesh "/Game/Cyberman/Mesh/SK_Jacket.SK_Jacket" true))
      (:`NewEnumerator4`
        (`SkinnedMeshComponent.SetSkinnedAssetAndUpdate` _skeletalmesh "/Game/Cyberman/Mesh/SK_Sheath.SK_Sheath" true)))))