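; Printing press actor that becomes triggerable by the player after the boss dies.
; A looping one-second timer polls the ClicheGameMode BossDeath flag, then enables collision on the trigger Box and clears itself.
; The first overlap by an actor tagged HeroPlayer plays a sound from an offset start time and starts the press's many component animations together, without looping.
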(event `self.ReceiveBeginPlay`
  (bind _returnvalue (`KismetSystemLibrary.K2_SetTimerDelegate` (delegate `CheckBossDeath`) 1.0 true))
  (set `self.CheckBossHandle` _returnvalue))

(event `CheckBossDeath`
  (bind _ascliche_game_mode (cast `/Game/Blueprints/GameMode/ClicheGameMode` (`GameplayStatics.GetGameMode`)))
  (if (`/Game/Blueprints/GameMode/ClicheGameMode.BossDeath` _ascliche_game_mode)
    (`/Engine/EditorBlueprintResources/StandardMacros.DoOnce` false
      (:`Completed`
        (`PrimitiveComponent.SetCollisionEnabled` (`self.Box`) "QueryAndPhysics")
        (`KismetSystemLibrary.K2_ClearAndInvalidateTimerHandle` (`self.CheckBossHandle`))))))

(event `Activate Printer`
  (`SkeletalMeshComponent.Play` (`self.demo_旋转_3`) false)
  (`SkeletalMeshComponent.Play` (`self.demo_克隆_1_3`) false)
  (`SkeletalMeshComponent.Play` (`self.demo_对称`) false)
  (`SkeletalMeshComponent.Play` (`self.demo_克隆_1`) false)
  (`SkeletalMeshComponent.Play` (`self.demo_Tube`) false)
  (`SkeletalMeshComponent.Play` (`self.demo_notice`) false)
  (`SkeletalMeshComponent.Play` (`self.demo_Cylinder_1`) false)
  (`SkeletalMeshComponent.Play` (`self.demo_Cube_15`) false)
  (`SkeletalMeshComponent.Play` (`self.demo_克隆_1_2`) false)
  (`SkeletalMeshComponent.Play` (`self.demo_胶囊_3`) false)
  (`SkeletalMeshComponent.Play` (`self.demo_胶囊_2`) false)
  (`SkeletalMeshComponent.Play` (`self.demo_胶囊_1`) false)
  (`SkeletalMeshComponent.Play` (`self.demo_胶囊`) false)
  (`SkeletalMeshComponent.Play` (`self.demo_细分曲面_1`) false)
  (`SkeletalMeshComponent.Play` (`self.demo_管道_3`) false)
  (`SkeletalMeshComponent.Play` (`self.demo_立方体_1_5`) false)
  (`SkeletalMeshComponent.Play` (`self.demo_空白`) false))

(event `self.Box.OnComponentBeginOverlap`
  (params (OverlappedComponent :type "PrimitiveComponent Object Reference") (OtherActor :type "Actor Object Reference") (OtherComp :type "PrimitiveComponent Object Reference") (OtherBodyIndex :type Integer) (bFromSweep :type Boolean) (SweepResult :type "HitResult Structure (by ref)"))
  (if (`self.ActorHasTag` OtherActor "HeroPlayer")
    (`/Engine/EditorBlueprintResources/StandardMacros.DoOnce` false
      (:`Completed`
        (`GameplayStatics.PlaySoundAtLocation` "/Game/Blueprints/Sounds/MEDS_Large_Crossover_Short.MEDS_Large_Crossover_Short" (`self.K2_GetActorLocation`) (struct) 1.0 1.0 3.3 null null null null)
        (`self.Activate Printer`)))))

(fn `UserConstructionScript`)