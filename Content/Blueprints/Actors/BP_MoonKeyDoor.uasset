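; BP_MoonKeyDoor is a key pickup actor that, despite the "Door" in its name, contains no door logic.
; When an actor tagged HeroPlayer overlaps GrabTrigger, a DoOnce lets the grab run a single time.
; It adds a key enum entry to the HeroCharacter's inventory Keys map, shows the green key on the HUD_MainCharacter widget, then destroys itself.
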(event `self.GrabTrigger.OnComponentBeginOverlap`
  (params (OverlappedComponent :type "PrimitiveComponent Object Reference") (OtherActor :type "Actor Object Reference") (OtherComp :type "PrimitiveComponent Object Reference") (OtherBodyIndex :type Integer) (bFromSweep :type Boolean) (SweepResult :type "HitResult Structure (by ref)"))
  (if (`self.ActorHasTag` OtherActor "HeroPlayer")
    (`/Engine/EditorBlueprintResources/StandardMacros.DoOnce` false
      (:`Completed`
        (bind _ashero_character (cast `/Game/Blueprints/Characters/BaseClasses/HeroCharacter` OtherActor))
        (`BlueprintMapLibrary.Map_Add` (`.Keys_4_3AD3410D406BE811A81684A246E373C3` (break `/Game/Blueprints/Characters/MainHeroe/Structs/Inventory_Struct` (`/Game/Blueprints/Characters/BaseClasses/HeroCharacter.Inventory` _ashero_character))) "NewEnumerator0" true)
        (`/Game/Blueprints/HUD/HUD_MainCharacter.ShowGreenKey` (cast `/Game/Blueprints/HUD/HUD_MainCharacter` (`/Game/Blueprints/Characters/BaseClasses/HeroCharacter.HealthWidgetReference` _ashero_character) :!pure true))
        (`self.K2_DestroyActor`)))))

(fn `UserConstructionScript`)