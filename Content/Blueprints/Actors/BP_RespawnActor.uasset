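; Respawn volume that sends the hero back to their last stored location when they enter its box.
; On overlap by an actor tagged HeroPlayer, it casts to HeroCharacter, zeroes movement velocity and sets the location to LastPlayerLocation without a sweep.
; A DoOnce gates the response and is reset through RestartDoOnce right after the relocation.
; The construction script sizes the box from the RespawnExtend variable.
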(event `self.Box.OnComponentBeginOverlap`
  (params (OverlappedComponent :type "PrimitiveComponent Object Reference") (OtherActor :type "Actor Object Reference") (OtherComp :type "PrimitiveComponent Object Reference") (OtherBodyIndex :type Integer) (bFromSweep :type Boolean) (SweepResult :type "HitResult Structure (by ref)"))
  (if (`self.ActorHasTag` OtherActor "HeroPlayer")
    (`/Engine/EditorBlueprintResources/StandardMacros.DoOnce` false :!label _label
      (:`Completed`
        (bind _ashero_character (cast `/Game/Blueprints/Characters/BaseClasses/HeroCharacter` OtherActor)
          (:`then`
            (set `MovementComponent.Velocity` (0.0 0.0 0.0) (`Character.CharacterMovement` _ashero_character))
            (`self.K2_SetActorLocation` _ashero_character (`/Game/Blueprints/Characters/BaseClasses/HeroCharacter.LastPlayerLocation` _ashero_character) false false))
          (:`CastFailed`
            _))
        (`self.RestartDoOnce`)))))

(event `RestartDoOnce`
  (goto _label :!via `Reset`))

(fn `UserConstructionScript`
  (`BoxComponent.SetBoxExtent` (`self.Box`) (`self.RespawnExtend`) true))