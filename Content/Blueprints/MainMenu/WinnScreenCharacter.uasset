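; Win screen character that shows the win menu with a fade-in when play begins.
; BeginPlay creates the WinScreenWidget, shows the mouse cursor and switches input to UI only.
; A timeline drives both the camera's post-process gain and the widget's color and opacity.
; CloseMenu reverses the timeline to fade both back out, without removing the widget.
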(event `self.ReceiveBeginPlay`
  (bind _returnvalue (`GameplayStatics.GetPlayerController` 0))
  (bind _returnvalue_2 (`|CreateWidget` "/Game/Blueprints/MainMenu/WinScreenWidget.WinScreenWidget_C"))
  (bind _output_get (set `self.MenuWidget` _returnvalue_2))
  (`UserWidget.AddToViewport` _output_get 0)
  (set `PlayerController.bShowMouseCursor` true _returnvalue)
  (`WidgetBlueprintLibrary.SetInputMode_UIOnlyEx` _returnvalue null)
  (bind (_direction _timelapse) (`Timeline|Timeline_0` :!via `PlayFromStart` :!label _label)
    (:`Update`
      (setmembers `PostProcessSettings` :`StructRef` (`CameraComponent.PostProcessSettings` (`self.Camera`)) :`ColorGain` (`KismetMathLibrary.MakeVector4` 1.0 1.0 1.0 _timelapse))
      (`UserWidget.SetColorAndOpacity` (`self.MenuWidget`) (make `LinearColor` _timelapse _timelapse _timelapse _timelapse)))))

(event `CloseMenu`
  (goto _label :!via `Reverse`))

(fn `UserConstructionScript`)